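; Enemy character with HP and SP pools, basic chase and attack events, and getters for stats and mesh.
; Damage drains SP first, absorbing the whole hit while any remains, then HP; Tick destroys the actor at zero HP.
; Hitting MC_BP damages the player through a DoOnce that never resets, and smash launches the enemy forward.
; AIMoveTo chase is marked for AI replacement; Attack and Chaseplayer are empty stubs.
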(event `chaseplayer2D`
  ;[1 1 1] chase（replace by AI)
  (`|AIMoveTo` self (0.0 0.0 0.0) (`GameplayStatics.GetPlayerCharacter` 0)
    (:`OnSuccess`
      (`KismetSystemLibrary.Delay` 2.0)
      (`self.Attack`)
      (`self.chaseplayer`))))

(event `self.ReceiveBeginPlay`
  ;[1 1 1] damage
  (set `self.HP` (`self.HP Max`))
  (set `self.SP` (`self.SP MAX`)))

(event `self.ReceiveTick`
  (params (DeltaSeconds :type "Float (single-precision)"))
  ;[1 1 1] damage
  (`/Engine/EditorBlueprintResources/StandardMacros.IsValid` self
    (:`Is Valid`
      (if (<= (`self.HP`) 0.0)
        (`self.K2_DestroyActor`)))))

(event `self.ReceiveAnyDamage`
  (params (Damage :type "Float (single-precision)") (DamageType :type "DamageType Object Reference") (InstigatedBy :type "Controller Object Reference") (DamageCauser :type "Actor Object Reference"))
  ;[1 1 1] damage
  (`self.Damage` Damage Damage))

(event `Attack`)

(event `Attack2D`
  ;[1 1 1] Attack
  (`|PlayMontage` (`self.Mesh`)))

(event `self.ReceiveHit`
  (params (MyComp :type "PrimitiveComponent Object Reference") (Other :type "Actor Object Reference") (OtherComp :type "PrimitiveComponent Object Reference") (bSelfMoved :type Boolean) (HitLocation :type "Vector Structure") (HitNormal :type "Vector Structure") (NormalImpulse :type "Vector Structure") (Hit :type "HitResult Structure (by ref)"))
  ;[1 1 1] smash/hit
  (cast `/Game/ThirdPerson/Blueprints/Animations/MC_BP` Other)
  (`/Engine/EditorBlueprintResources/StandardMacros.DoOnce` false
    (:`Completed`
      (`GameplayStatics.ApplyDamage` (`GameplayStatics.GetPlayerCharacter` 0) 10.0))))

(event `smash`
  ;[1 1 1] smash/hit
  (`self.LaunchCharacter` (* (`self.GetActorForwardVector`) 1000.0)))

(fn `chaseplayer`)

(fn `Damage`
  (params (Damage :type "Float (double-precision)") (B2 :type "Float (double-precision)"))
  (locals (LocalDamage :type "Float (double-precision)"))
  (set `local.LocalDamage` Damage)
  (`|ExecutionSequence`
    (:`then_0`
      (if (> (`self.SP`) 0.0)
        (set `self.SP` (- (`self.SP`) (`KismetMathLibrary.FMin` (`self.SP`) (`local.LocalDamage`))))
        (set `local.LocalDamage` 0.0)))
    (:`then_1`
      (set `self.HP` (- (`self.HP`) (`local.LocalDamage`))))))

(fn `Get Body`
  (returns (body :type "SkeletalMeshComponent Object Reference"))
  (return (`self.Mesh`)))

(fn `Get HP`
  (returns (HP :type "Float (double-precision)"))
  (return (`self.HP`)))

(fn `Get HP Max`
  (returns (`HP Max` :type "Float (double-precision)"))
  (return (`self.HP MAX`)))

(fn `Get SP`
  (returns (SP :type "Float (double-precision)"))
  (return (`self.SP`)))

(fn `Get SP Max`
  (returns (`SP Max` :type "Float (double-precision)"))
  (return (`self.SP MAX`)))

(fn `UserConstructionScript`)